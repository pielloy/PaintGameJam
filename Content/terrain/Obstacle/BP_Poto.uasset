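; BP_Poto is a terrain obstacle that grows on demand, with a growing-plant sound.
; CallGrow responds to one enum type by playing the sound at the actor and starting a looping timer on Grow.
; Each Grow tick adds Speed to Scale and applies it to the Arrow component, clearing the timer once X reaches full scale.
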(fn `CallGrow`
  (params (Type :type "/Game/player/E_Elements Enum" :default "NewEnumerator0"))
  (if (`|EnumEquality` Type "NewEnumerator1")
    (`KismetSystemLibrary.K2_SetTimer` self "Grow" 0.05 true)
    (`GameplayStatics.PlaySoundAtLocation` "/Game/sounds/interaction/planteQuiPousse.planteQuiPousse" (`self.K2_GetActorLocation`) (struct) 0.2 1.0 0.0 null null null)))

(fn `Grow`
  (bind _scale_x (`KismetMathLibrary.BreakVector` (`self.scale`)))
  (bind _output_get (set `self.scale` (+ (`self.scale`) (`self.speed`))))
  (`SceneComponent.SetRelativeScale3D` (`self.Arrow`) _output_get)
  (if (>= _scale_x 1.0)
    (`KismetSystemLibrary.K2_ClearTimer` self "Grow")))

(fn `UserConstructionScript`)